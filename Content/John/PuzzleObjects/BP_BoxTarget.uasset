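; BP_BoxTarget is a puzzle target that plays the DoorOpening2 level sequence when a BP_MovableBox's Cube overlaps its Box trigger.
; BeginPlay gives the target's Cube a dynamic M_Box material with raised intensity and a color set on an unnamed parameter.
; Overlap begin and end toggle the box's Target flag.
; The end-overlap color change never runs because it checks Target just after clearing it.
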(event `self.ReceiveBeginPlay`
  (bind _cube (`self.Cube`))
  (bind _returnvalue (`PrimitiveComponent.CreateDynamicMaterialInstance` _cube 0 "/Game/John/PuzzleObjects/M_Box.M_Box" "None"))
  (`PrimitiveComponent.SetMaterial` _cube 0 _returnvalue)
  (`MaterialInstanceDynamic.SetScalarParameterValue` _returnvalue "Intensity" 20.0)
  (`MaterialInstanceDynamic.SetVectorParameterValue` _returnvalue "None" (struct :`R` 0.392708 :`G` 0.013724)))

(event `self.Box.OnComponentBeginOverlap`
  (params (OverlappedComponent :type "PrimitiveComponent Object Reference") (OtherActor :type "Actor Object Reference") (OtherComp :type "PrimitiveComponent Object Reference") (OtherBodyIndex :type Integer) (bFromSweep :type Boolean) (SweepResult :type "HitResult Structure (by ref)"))
  (bind _asbp_movable_box (cast `/Game/John/PuzzleObjects/BP_MovableBox` OtherActor))
  (set `/Game/John/PuzzleObjects/BP_MovableBox.Target?` true _asbp_movable_box)
  (if (== OtherComp (`/Game/John/PuzzleObjects/BP_MovableBox.Cube` _asbp_movable_box))
    (if (`/Game/John/PuzzleObjects/BP_MovableBox.Target?` _asbp_movable_box)
      (bind (_outactor _returnvalue) (`LevelSequencePlayer.CreateLevelSequencePlayer` "/Game/John/PuzzleObjects/DoorAnimations/DoorOpening/DoorOpening2.DoorOpening2"))
      (`MovieSceneSequencePlayer.Play` _returnvalue))))

(event `self.Box.OnComponentEndOverlap`
  (params (OverlappedComponent :type "PrimitiveComponent Object Reference") (OtherActor :type "Actor Object Reference") (OtherComp :type "PrimitiveComponent Object Reference") (OtherBodyIndex :type Integer))
  (bind _asbp_movable_box (cast `/Game/John/PuzzleObjects/BP_MovableBox` OtherActor))
  (set `/Game/John/PuzzleObjects/BP_MovableBox.Target?` false _asbp_movable_box)
  (if (== OtherComp (`/Game/John/PuzzleObjects/BP_MovableBox.Cube` _asbp_movable_box))
    (if (`/Game/John/PuzzleObjects/BP_MovableBox.Target?` _asbp_movable_box)
      (`MaterialInstanceDynamic.SetVectorParameterValue` (stale `self.ReceiveBeginPlay` _returnvalue) "None" (struct :`R` 0.458333 :`B` 0.013226)))))

(fn `UserConstructionScript`)